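; BP_DwarfGamemode is a game mode that sets up local players and splits them into Red and Blue dwarf teams.
; On BeginPlay it calls CreatePlayer for two indices, then sets the default pawn class to BP_Player.
; It then gathers all PlayerEntityController actors, alternates their team by array index, and calls StartNewPlayer on each.
; An unconnected controller spawn node never runs, and Tick is unused.
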(event `self.ReceiveBeginPlay`
  (for _index (range 2)
    (`GameplayStatics.CreatePlayer` _index))
  (set `self.DefaultPawnClass` "/Game/Blueprints/Players/BP_Player.BP_Player_C")
  (bind _outactors (`GameplayStatics.GetAllActorsOfClass` "/Script/Dwarf_Game_DES310.PlayerEntityController"))
  (for (_array_element _array_index) _outactors
    (if (== (mod _array_index 2) 0)
      (`PlayerEntityController.SetTeamType` _array_element "RedDwarf")
      (else
        (`PlayerEntityController.SetTeamType` _array_element "BlueDwarf")))
    (`self.StartNewPlayer` _array_element)))

(fn `UserConstructionScript`)