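; BP_Forge is a forge world object with a fire effect, a spot light and a point light, switchable between blue and orange flames.
; The construction script picks two colours from the IsBlue flag and passes them to the Fire effect's FirstColour and SecondColour variables.
; Both lights take the primary colour, so their glow matches the flame.
; The event graph has no active logic.
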(fn `UserConstructionScript`
  (bind _fire (`self.Fire`))
  (bind _particlecolor1 (`self.ParticleColor1`))
  (`|ExecutionSequence`
    (:`then_0`
      (if (`self.IsBlue`)
        (set `self.ParticleColor1` (struct :`R` 0.011765 :`G` 0.380392 :`B` 1.0 :`A` 1.0))
        (set `self.ParticleColor2` (struct :`R` 0.002104 :`G` 0.049577 :`B` 0.65625 :`A` 1.0))
        (else
          (set `self.ParticleColor1` (struct :`R` 1.0 :`G` 0.188235 :`B` 0.027451 :`A` 1.0))
          (set `self.ParticleColor2` (struct :`R` 1.0 :`G` 0.532413 :`A` 1.0))))
      (`NiagaraComponent.SetVariableLinearColor` _fire "FirstColour" (`self.ParticleColor1`))
      (`NiagaraComponent.SetVariableLinearColor` _fire "SecondColour" (`self.ParticleColor2`))
      (`LightComponent.SetLightColor` (`self.SpotLight`) _particlecolor1 true)
      (`LightComponent.SetLightColor` (`self.PointLight`) _particlecolor1 true))))