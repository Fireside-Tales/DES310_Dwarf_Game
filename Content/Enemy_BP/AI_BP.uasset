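; AI controller for the Wisp enemy, running an Idle/Moving/Attacking state machine on Tick while the possessed pawn is alive.
; Idle switches to Moving on a timer or player sighting; Moving chases the player or picks random navmesh points.
; An attack check compares the actors' distances from world origin, rather than their separation, to enter Attacking and raise walk speed.
; Attacking keeps chasing only while the Wisp's attack and movement flags allow.
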(event `self.ReceivePossess`
  (params (PossessedPawn :type "Pawn Object Reference"))
  (bind _aswisp_ai_bp (cast `/Game/Enemy_BP/Wisp_AI_BP` PossessedPawn))
  (set `self.Wisp` _aswisp_ai_bp))

(event `self.ReceiveTick`
  (params (DeltaSeconds :type "Float (single-precision)"))
  (bind _wisp (`self.Wisp`))
  (bind _wisp_2 (`self.Wisp`))
  (if (`AI_Actor.mb_isAlive` (`self.Wisp`))
    (`KismetSystemLibrary.PrintString` (`|GetEnumeratorNameAsString` (`Base_Enemy.m_EnemyStates` (`self.Wisp`))) true true (struct :`R` 1.0 :`B` 0.177487 :`A` 1.0) 0.1)
    (`self.Swich to attack state`)
    (`/Engine/EditorBlueprintResources/StandardMacros.IsValid` _wisp
      (:`Is Valid`
        (switch `EnemyStates` (`Base_Enemy.m_EnemyStates` _wisp)
          (:`Idle`
            ;[1 1 1] Handles when the wisp should move
            (`|ExecutionSequence`
              (:`then_0`
                (bind _output_get (set `self.Move Timer` (+ (`self.Move Timer`) (`GameplayStatics.GetWorldDeltaSeconds`))))
                (if (> _output_get (`self.Timer Target`))
                  (set `Base_Enemy.m_EnemyStates` "Moving" (`self.Wisp`))))
              (:`then_1`
                (if (`/Game/Enemy_BP/Wisp_AI_BP.Can See Player` (`self.Wisp`))
                  (set `Base_Enemy.m_EnemyStates` "Moving" (`self.Wisp`))
                  (`KismetSystemLibrary.PrintString` "I SEE PLAYER")))))
          (:`Moving`
            ;[1 1 1] Moving
            (if (`/Game/Enemy_BP/Wisp_AI_BP.Can See Player` (`self.Wisp`))
              (`self.Move towards player`)
              (else
                (`self.Random Movement`))))
          (:`Attacking`
            (if (and (`/Game/Enemy_BP/Wisp_AI_BP.AttackPlayer` _wisp_2) (`/Game/Enemy_BP/Wisp_AI_BP.Still Move` _wisp_2))
              (`self.Move towards player`))))))))

(event `Move towards player`
  ;[1 1 1] Handles the tracking of the player
  (`|AIMoveTo` null (`self.K2_GetActorLocation` (`GameplayStatics.GetPlayerCharacter` 0)) null 0.0))

(event `Random Movement`
  ;[1 1 1] Handles the movement of the AI When not tracking the Player
  (if (not (`self.NewLocationSet`))
    (`|AIMoveTo` null (`NavigationSystemV1.K2_GetRandomLocationInNavigableRadius` (`self.K2_GetActorLocation` (`self.Wisp`)) (`self.Acceptance Radius`) null null) null 50.0
      (:`then`
        (set `self.Timer Target` 5.0)
        (set `self.NewLocationSet` true))
      (:`OnSuccess`
        (set `self.Timer Target` (`KismetMathLibrary.RandomFloatInRange` 1.0 5.0))
        (set `self.Move Timer` 0.0)
        (set `self.NewLocationSet` false)
        (set `Base_Enemy.m_EnemyStates` "Idle" (`self.Wisp`)))
      (:`OnFail`
        (set `self.Timer Target` 5.0)
        (set `self.NewLocationSet` false)))))

(event `Swich to attack state`
  (bind _wisp (`self.Wisp`))
  (bind _wisp_2 (`self.Wisp`))
  (bind _player_ref (`/Game/Enemy_BP/Wisp_AI_BP.Player Ref` _wisp))
  ;[1 1 1] Checks if it is range to attack the player
  (`/Engine/EditorBlueprintResources/StandardMacros.IsValid` _player_ref
    (:`Is Valid`
      (if (< (`KismetMathLibrary.Abs` (- (`KismetMathLibrary.VSize` (`self.K2_GetActorLocation` _wisp)) (`KismetMathLibrary.VSize` (`self.K2_GetActorLocation` _player_ref)))) 100.0)
        (set `Base_Enemy.m_EnemyStates` "Attacking" (`self.Wisp`))
        (set `CharacterMovementComponent.MaxWalkSpeed` 1000.0 (`Character.CharacterMovement` _wisp_2))
        (if (not (`/Game/Enemy_BP/Wisp_AI_BP.AttackPlayer` _wisp_2))
          (`NavMovementComponent.StopActiveMovement` (`Character.CharacterMovement` (`self.Wisp`))))
        (else
          (`self.Reset Enemy`))))))

(event `Reset Enemy`
  (bind _wisp (`self.Wisp`))
  (if (`|EnumInequality` (`Base_Enemy.m_EnemyStates` _wisp) "Attacking")
    (set `CharacterMovementComponent.MaxWalkSpeed` 600.0 (`Character.CharacterMovement` _wisp))
    (set `/Game/Enemy_BP/Wisp_AI_BP.Still Move` true (`self.Wisp`))))

(fn `UserConstructionScript`)