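; Collectible pickup Blueprint with three types: Max Health, Move Speed and Strength.
; The Construction Script sets rotation and bounce speeds, then switches on the type to assign a colored crystal mesh and a collect value.
; On actor overlap it only adds an audio component; the Player_Character cast is disconnected, and the graph applies no stat or motion.
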(event `self.ReceiveActorBeginOverlap`
  (params (OtherActor :type "Actor Object Reference"))
  (`AddComponent|NODE_AddAudioComponent-0`))

(fn `UserConstructionScript`
  (bind _m_mesh (`self.m_Mesh`))
  (set `self.rotationSpeed` 30.0)
  (set `self.bounceSpeed` 5.0)
  (switch `CollectibleType` (`self.m_CollectibleType`)
    (:`MaxHealth`
      (`StaticMeshComponent.SetStaticMesh` _m_mesh "/Game/Collectables/Collectible_Assets/CrystalGreen.CrystalGreen")
      (set `self.mf_CollectValue` 10.0))
    (:`MoveSpeed`
      (`StaticMeshComponent.SetStaticMesh` _m_mesh "/Game/Collectables/Collectible_Assets/CrystalPurple.CrystalPurple")
      (set `self.mf_CollectValue` 10.0))
    (:`Strength`
      (`StaticMeshComponent.SetStaticMesh` _m_mesh "/Game/Collectables/Collectible_Assets/CrystalOrange.CrystalOrange")
      (set `self.mf_CollectValue` 100.0))))