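; Player character Blueprint that moves, looks around, and aims, throws and recalls a returning pickaxe.
; BeginPlay attaches the child-actor Pickaxe to the hand socket, passes it player and camera references, and initializes it.
; Aiming plays a camera-lerp timeline that reverses on release, while throwing detaches and launches the axe on a montage notify.
; A DoOnce gates recall until Catch hands the mesh to the axe and resets it, and Tick runs player-state handling.
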(event `self.ReceiveTick`
  (params (DeltaSeconds :type "Float (single-precision)"))
  (`self.HandlePlayerStates`))

(event `self.ReceiveBeginPlay`
  (bind _axe_ref (`self.Axe Ref`))
  (bind _aspickaxe (cast `/Game/Weapon/Pickaxe` (`ChildActorComponent.ChildActor` (`self.m_Pickaxe`))))
  (`|ExecutionSequence`
    (:`then_0`
      (set `self.Axe Ref` _aspickaxe))
    (:`then_1`
      (set `PickaxeProjectile.playerRef` self _aspickaxe)
      (`SceneComponent.K2_AttachToComponent` (`self.m_Pickaxe`) (`self.Mesh`) "HandSocket" "SnapToTarget" "SnapToTarget" "KeepWorld" true))
    (:`then_2`
      (bind _output_get (set `PickaxeProjectile.m_Camera` (`self.camera`) _aspickaxe))
      (`PickaxeProjectile.InitVariables` _axe_ref (`PickaxeProjectile.PickMovement` _axe_ref) (`/Game/Weapon/Master_Pick.Pivot_Point` _axe_ref) (`/Game/Weapon/Master_Pick.Lodge_Point` _axe_ref) _output_get))))

(event `InputAxis|Move Forward / Backward`
  (params (AxisValue :type "Float (single-precision)"))
  (bind (_returnvalue_roll _returnvalue_pitch _returnvalue_yaw) (`KismetMathLibrary.BreakRotator` (`self.GetControlRotation`)))
  ;[1 1 1] Character Movement
  (`self.AddMovementInput` (`KismetMathLibrary.GetForwardVector` (`KismetMathLibrary.MakeRotator` 0.0 0.0 _returnvalue_yaw)) AxisValue true))

(event `InputAxis|Move Right / Left`
  (params (AxisValue :type "Float (single-precision)"))
  (bind (_returnvalue_roll _returnvalue_pitch _returnvalue_yaw) (`KismetMathLibrary.BreakRotator` (`self.GetControlRotation`)))
  ;[1 1 1] Character Movement
  (`self.AddMovementInput` (`KismetMathLibrary.GetRightVector` (`KismetMathLibrary.MakeRotator` _returnvalue_roll 0.0 _returnvalue_yaw)) AxisValue true))

(event `InputAction|Throw`
  (params (Key :type "Key Structure"))
  (:`Pressed`
    (if (`self.mb_Aiming`)
      (`self.Throw Axe BP`))))

(event `InputAxis|Turn Right / Left Mouse`
  (params (AxisValue :type "Float (single-precision)"))
  ;[1 1 1] Rotation on the camera
  (`self.AddControllerYawInput` AxisValue))

(event `InputAxis|Look Up / Down Mouse`
  (params (AxisValue :type "Float (single-precision)"))
  ;[1 1 1] Rotation on the camera
  (`self.AddControllerPitchInput` AxisValue))

(event `InputAction|Recall`
  (params (Key :type "Key Structure"))
  (:`Pressed`
    (if (`PickaxeProjectile.mb_Thrown` (`self.Axe Ref`))
      (`self.Recall event`))))

(event `InputAxis|Look Up / Down Gamepad`
  (params (AxisValue :type "Float (single-precision)"))
  (`self.AddControllerYawInput` AxisValue))

(event `InputAxis|Turn Right / Left Gamepad`
  (params (AxisValue :type "Float (single-precision)"))
  (`self.AddControllerPitchInput` AxisValue))

(event `InputAction|Aim`
  (params (Key :type "Key Structure"))
  (bind _cameralerp (`self.CameraLerp`))
  ;[1 1 1] this handles the aiming of the axe for the player
  (:`Pressed`
    (`self.Aim`)
    (`TimelineComponent.SetPlayRate` _cameralerp 1.4)
    (bind (_direction _lerp_curve) (`Timeline|CameraLerp` :!label _label)
      (:`Update`
        (`self.LerpCamera` _lerp_curve))))
  (:`Released`
    (`self.ReleaseAim`)
    (`TimelineComponent.SetPlayRate` _cameralerp 0.9)
    (goto _label :!via `Reverse`)))

(event `Throw Axe BP`
  (bind _axe_ref (`self.Axe Ref`))
  ;[1 1 1] Handle the axe throw
  (if (not (`PickaxeProjectile.mb_Thrown` (`self.Axe Ref`)))
    (set `self.m_PlayerStates` "Throwing")
    (`KismetSystemLibrary.PrintString` "Hello")
    (`|PlayMontage` (`self.Mesh`) "/Game/Animation/Dwarf/Animation/High_PolyThrow.High_PolyThrow"
      (:`OnNotifyBegin`
        (`self.K2_DetachFromActor` _axe_ref "KeepWorld" "KeepWorld" "KeepWorld")
        (`/Game/Weapon/Pickaxe.Throw` _axe_ref)))))

(event `Recall event`
  (`/Engine/EditorBlueprintResources/StandardMacros.DoOnce` false :!label _label_2
    (:`Completed`
      (`/Game/Weapon/Pickaxe.Recall` (`self.Axe Ref`))
      (`KismetSystemLibrary.PrintString` "Hello"))))

(event `Catch`
  (`PickaxeProjectile.Catch` (`self.Axe Ref`) (`self.Mesh`))
  (`|ExecutionSequence`
    (:`then_0`
      (goto _label_2 :!via `Reset`))))

(fn `UserConstructionScript`)