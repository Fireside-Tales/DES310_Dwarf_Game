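; Player character Blueprint for a dwarf who moves, dashes, throws and recalls a pickaxe, and can carry an heirloom.
; BeginPlay attaches and initializes the child-actor axe; catching it snaps any attached heirloom to the player.
; Possession creates the HUD and a looping timer that toggles a custom-depth outline post-process on heirloom carriers by distance.
; Tick gathers other players, updates dash and timeline-driven FOV, and runs the respawn timer; aiming lerps the camera.
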(event `self.ReceiveBeginPlay`
  ;[1 1 1] Handles all the stuff that should be done on the begin play
  (`|ExecutionSequence`
    (:`then_1`
      ;;[1 1 1] this is where it sets up the heirloom reference
      (bind _outactors (`GameplayStatics.GetAllActorsOfClass` "/Game/Collectables/Heirloom_BP.Heirloom_BP_C"))
      (for _array_element _outactors
        (set `self.m_heirloom` _array_element)))
    (:`then_2`
      (bind _aspickaxe (cast `/Game/Weapon/Pickaxe` (`ChildActorComponent.ChildActor` (`self.m_Pickaxe`))))
      (`|ExecutionSequence`
        (:`then_0`
          ;;[1 1 1] Sets the players Reference for the axe and the reference of the player to the axe
          (set `self.m_AxeRef` _aspickaxe))
        (:`then_1`
          (set `PickaxeProjectile.playerRef` self _aspickaxe)
          ;;[1 1 1] attaches the axe to the players hand
          (`SceneComponent.K2_AttachToComponent` (`self.m_Pickaxe`) (`self.Mesh`) "HandSocket" "SnapToTarget" "SnapToTarget" "KeepWorld" true))
        (:`then_2`
          (bind _aspickaxe_2 (cast `/Game/Weapon/Pickaxe` (`self.m_AxeRef`)))
          (bind _output_get (set `PickaxeProjectile.m_Camera` (`self.camera`) _aspickaxe))
          (`PickaxeProjectile.InitVariables` _aspickaxe_2 (`PickaxeProjectile.PickMovement` _aspickaxe_2) (`/Game/Weapon/Master_Pick.Pivot_Point` _aspickaxe_2) (`/Game/Weapon/Master_Pick.Lodge_Point` _aspickaxe_2) _output_get))))))

(event `self.ReceivePossessed`
  (params (NewController :type "Controller Object Reference"))
  ;[1 1 1] Player HUD setup
  (`self.Create Player Hud`)
  (`self.Make Post Processing Effect`)
  (castclass `/Game/Assets/Low_Poly_Dwarf/Dwarf_Animation_BP` null))

(event `Create Player Hud`
  ;[1 1 1] Player HUD setup
  (bind _asplayer_controller (cast `PlayerController` (`self.GetController`)))
  (bind _returnvalue (`|CreateWidget` "/Game/UI/PlayerHud.PlayerHud_C" _asplayer_controller))
  (`UserWidget.AddToPlayerScreen` _returnvalue 0))

(event `InputAxis|Move Forward / Backward`
  (params (AxisValue :type "Float (single-precision)"))
  (bind (_returnvalue_roll _returnvalue_pitch _returnvalue_yaw) (`KismetMathLibrary.BreakRotator` (`self.GetControlRotation`)))
  ;[1 1 1] Character Movement
  (if (`self.Invalid Player States Moving`)
    (`self.AddMovementInput` (`KismetMathLibrary.GetForwardVector` (`KismetMathLibrary.MakeRotator` 0.0 0.0 _returnvalue_yaw)) AxisValue true)))

(event `InputAxis|Move Right / Left`
  (params (AxisValue :type "Float (single-precision)"))
  (bind (_returnvalue_roll _returnvalue_pitch _returnvalue_yaw) (`KismetMathLibrary.BreakRotator` (`self.GetControlRotation`)))
  ;[1 1 1] Character Movement
  (if (`self.Invalid Player States Moving`)
    (`self.AddMovementInput` (`KismetMathLibrary.GetRightVector` (`KismetMathLibrary.MakeRotator` _returnvalue_roll 0.0 _returnvalue_yaw)) AxisValue true)))

(event `InputAction|Recall`
  (params (Key :type "Key Structure"))
  ;[1 1 1] Handles the inputs for recalling the axe
  (:`Pressed`
    (if (`PickaxeProjectile.mb_Thrown` (`self.m_AxeRef`))
      (`self.Recall event`))))

(event `FOVChange`
  ;[1 1 1] Adjusts theFOV when running
  (if (`self.mb_isDashing`)
    (bind (_direction _fov) (`Timeline|ChangeOverTime` :!label _label)
      (:`Update`
        (`CameraComponent.SetFieldOfView` (`self.camera`) _fov)))
    (else
      (goto _label :!via `Reverse`))))

(event `InputAxis|Turn Right / Left Gamepad`
  (params (AxisValue :type "Float (single-precision)"))
  ;[1 1 1] Game Pad Turning
  (`self.AddControllerYawInput` (* AxisValue (`CameraSensitivityBPLibrary.GetHorizontalSensitivity`))))

(event `InputAxis|Turn Right / Left Mouse`
  (params (AxisValue :type "Float (single-precision)"))
  ;[1 1 1] Mouse Rotation
  (`self.AddControllerYawInput` AxisValue))

(event `InputAxis|Look Up / Down Mouse`
  (params (AxisValue :type "Float (single-precision)"))
  ;[1 1 1] Mouse Rotation
  (`self.AddControllerPitchInput` AxisValue))

(event `InputAxis|Look Up / Down Gamepad`
  (params (AxisValue :type "Float (single-precision)"))
  ;[1 1 1] Game Pad Turning
  (`self.AddControllerPitchInput` AxisValue))

(event `Key|Six`
  (params (Key :type "Key Structure"))
  (:`Pressed`
    (set `self.m_PlayerStats` (make `PlayerStats` false))))

(event `self.ReceiveTick`
  (params (DeltaSeconds :type "Float (single-precision)"))
  ;[1 1 1] Event Tick function
  (`|ExecutionSequence`
    (:`then_0`
      (if (not (`self.All Players Grabbed`))
        (`self.Get All Players`)))
    (:`then_1`
      (`self.PlayerDash` DeltaSeconds)
      (`self.FOVChange`)
      (`KismetSystemLibrary.PrintString` (`KismetStringLibrary.Conv_BoolToString` (`self.mb_HasHeirloom`)) true true (struct :`G` 0.66 :`B` 1.0 :`A` 1.0) 0.001))
    (:`then_2`
      (if (`self.Start Respawn Time`)
        (set `self.Respawn Timer` (+ DeltaSeconds (`self.Respawn Timer`)))
        (if (>= (`self.Respawn Timer`) (`self.timer Target`))
          (set `self.Start Respawn Time` false)
          (set `self.Respawn Timer` 0.0)
          (set `self.m_PlayerStates` "Respawning")
          (`self.RespawnPlayer`))))))

(event `Toggle Post Process`
  (bind _camera (`self.camera`))
  ;[1 1 1] Handles whether the post process should be used
  (for _array_element (`self.Player Refs`)
    (if (`Base_Player.mb_HasHeirloom` _array_element)
      (if (> (`KismetMathLibrary.Abs` (- (`KismetMathLibrary.VSize` (`self.K2_GetActorLocation`)) (`KismetMathLibrary.VSize` (`self.K2_GetActorLocation` _array_element)))) 500.0)
        (bind _mesh (`Character.Mesh` _array_element))
        (`PrimitiveComponent.SetRenderCustomDepth` _mesh true)
        (set `CameraComponent.PostProcessSettings` (`self.Post Process Settings`) _camera)
        (else
          (`PrimitiveComponent.SetRenderCustomDepth` _mesh false :!label _label_2)
          (set `CameraComponent.PostProcessSettings` (struct) _camera)))
      (else
        (goto _label_2)))))

(event `Make Post Processing Effect`
  ;[1 1 1] Handles whether the post process should be used
  (`KismetSystemLibrary.K2_SetTimerDelegate` (delegate `Toggle Post Process`) 0.5 true)
  (bind _returnvalue (`KismetMaterialLibrary.CreateDynamicMaterialInstance` "/Game/Post_Processing_Material/PlayerOutline.PlayerOutline"))
  (bind _output_get (set `self.Outline` _returnvalue))
  (set `self.Post Process Settings` (make `PostProcessSettings` :`WeightedBlendables` (make `WeightedBlendables` (`|MakeArray` (make `WeightedBlendable` 1.0 _output_get))))))

(event `InputAction|Aim`
  (params (Key :type "Key Structure"))
  (bind _cameralerp (`self.CameraLerp`))
  ;[1 1 1] this handles the aiming of the axe for the player
  (:`Pressed`
    (`self.Aim`)
    (`TimelineComponent.SetPlayRate` _cameralerp 1.4)
    (bind (_direction _lerp_curve) (`Timeline|CameraLerp` :!label _label)
      (:`Update`
        (`self.LerpCamera` _lerp_curve))))
  (:`Released`
    (`self.ReleaseAim`)
    (`TimelineComponent.SetPlayRate` _cameralerp 0.9)
    (goto _label :!via `Reverse`)))

(event `Throw Axe BP`
  (bind _m_axeref (`self.m_AxeRef`))
  ;[1 1 1] Handle the axe throw
  (`self.K2_DetachFromActor` _m_axeref "KeepWorld" "KeepWorld" "KeepWorld")
  (bind _aspickaxe (cast `/Game/Weapon/Pickaxe` _m_axeref))
  (`/Game/Weapon/Pickaxe.Throw` _aspickaxe))

(event `Recall event`
  (`/Engine/EditorBlueprintResources/StandardMacros.DoOnce` false :!label _label_2
    (:`Completed`
      (bind _aspickaxe (cast `/Game/Weapon/Pickaxe` (`self.m_AxeRef`)))
      (`/Game/Weapon/Pickaxe.Recall` _aspickaxe)
      (`KismetSystemLibrary.PrintString` "Hello"))))

(event `Catch`
  (bind _m_heirloom (`self.m_heirloom`))
  (bind _m_axeref (`self.m_AxeRef`))
  (`PickaxeProjectile.Catch` _m_axeref (`self.Mesh`))
  (`|ExecutionSequence`
    (:`then_0`
      (goto _label_2 :!via `Reset`))
    (:`then_1`
      (for _array_element (`self.GetAttachedActors` (`self.m_AxeRef`) true false)
        (if (== (`self.m_heirloom`) _array_element)
          (`self.K2_DetachFromActor` _m_heirloom "KeepWorld" "KeepWorld" "KeepWorld")
          (`Heirloom_Class.SnapToPlayer` _m_heirloom (`self.Mesh`) self))))
    (:`then_2`
      (bind _asmaster_pick (cast `/Game/Weapon/Master_Pick` _m_axeref))
      (`ActorComponent.Deactivate` (`/Game/Weapon/Master_Pick.Trail` _asmaster_pick)))))

(fn `Get All Players`
  ;[1 1 1] Grabs a reference to all the other players
  (bind _outactors (`GameplayStatics.GetAllActorsOfClass` "Player_Character_C"))
  (for _array_element _outactors
    (if (!= _array_element self)
      (`KismetArrayLibrary.Array_Add` (`self.Player Refs`) _array_element)))
  (set `self.All Players Grabbed` true))

(fn `UserConstructionScript`
  (set `self.m_PlayerStats` (make `PlayerStats` true 100.0 1.0 (`CharacterMovementComponent.MaxWalkSpeed` (`self.CharacterMovement`)) 10.0 1.75))
  (set `self.mf_StaminaTarget` 3.0))