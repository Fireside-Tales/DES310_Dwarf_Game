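; Player collection point actor that ends the game by quitting when its player reaches it carrying the heirloom.
; On the first Tick, SetPlayerGoals scans all Player_Character actors, caches the nearest as PlayerRef and sets IsSet to stop further searches.
; The Box overlap quits only if the overlapping actor is that cached player and MbHasHeirloom is true.
; Debug strings print during both search and overlap.
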(event `self.ReceiveBeginPlay`)

(event `self.ReceiveTick`
  (params (DeltaSeconds :type "Float (single-precision)"))
  (if (not (`self.isSet`))
    (`self.Set Player Goals`)))

(event `self.Box.OnComponentBeginOverlap`
  (params (OverlappedComponent :type "PrimitiveComponent Object Reference") (OtherActor :type "Actor Object Reference") (OtherComp :type "PrimitiveComponent Object Reference") (OtherBodyIndex :type Integer) (bFromSweep :type Boolean) (SweepResult :type "HitResult Structure (by ref)"))
  (`KismetSystemLibrary.PrintString` "Hello")
  (if (== OtherActor (`self.PlayerRef`))
    (if (`Base_Player.mb_HasHeirloom` (`self.PlayerRef`))
      (`KismetSystemLibrary.QuitGame` null "Quit"))))

(fn `Set Player Goals`
  (bind _playerref (`self.PlayerRef`))
  (bind _outactors (`GameplayStatics.GetAllActorsOfClass` "/Game/Player/Blueprints/Player_Character.Player_Character_C"))
  (`KismetSystemLibrary.PrintString` (`KismetStringLibrary.Conv_IntToString` (`KismetArrayLibrary.Array_Length` _outactors)) true true (struct :`G` 0.66 :`B` 1.0 :`A` 1.0) 5.0)
  (for _array_element _outactors
    (`/Engine/EditorBlueprintResources/StandardMacros.IsValid` _playerref
      (:`Is Valid`
        (`KismetSystemLibrary.PrintString` "Hello")
        (if (< (`KismetMathLibrary.Abs` (`self.GetDistanceTo` _array_element)) (`KismetMathLibrary.Abs` (`self.GetDistanceTo` _playerref)))
          (set `self.PlayerRef` _array_element)))
      (:`Is Not Valid`
        (set `self.PlayerRef` _array_element)
        (`KismetSystemLibrary.PrintString` "Not valid"))))
  (set `self.isSet` true))

(fn `UserConstructionScript`)